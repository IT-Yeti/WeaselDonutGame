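; Player pawn for the weasel, which swings on ropes in the Y-Z plane and jumps on a cooldown.
; AttachLine traces toward the deprojected mouse cursor and, on an "Attachable"-tagged hit, spawns a Rope and attaches the mesh to its cable end.
; Jump while hanging, or Detach, releases the rope with a sideways-upward push.
; BeginPlay creates HUD, win and lose widgets; a looping timer shows jump and DashAbility readiness.
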(event `InputAction|QuitGame`
  (params (Key :type "Key Structure"))
  (:`Pressed`
    (`KismetSystemLibrary.QuitGame` null "Quit")))

(event `self.ReceiveBeginPlay`
  (bind _returnvalue (`GameplayStatics.GetPlayerController` 0))
  (bind _returnvalue_2 (`GameplayStatics.GetPlayerController` 0))
  (bind _playerhud (`self.PlayerHud`))
  (set `PlayerController.bShowMouseCursor` true _returnvalue_2)
  (set `self.StartingLocation` (`self.K2_GetActorLocation` _returnvalue_2))
  (set `self.JumpTimer` 0.0)
  (bind _returnvalue_3 (`|CreateWidget` "/Game/Blueprints/WBP_PlayerHUD.WBP_PlayerHUD_C" (`GameplayStatics.GetPlayerController` 0)))
  (`UserWidget.AddToViewport` _returnvalue_3 0)
  (bind _output_get (set `self.PlayerHud` _returnvalue_3))
  (`/Game/Blueprints/WBP_PlayerHUD.DashNotAvalaible` _playerhud)
  (`/Game/Blueprints/WBP_PlayerHUD.DashNotAvalaible` _output_get)
  (`/Game/Blueprints/WBP_PlayerHUD.JumpNotAvalaible` _playerhud)
  (bind _returnvalue_4 (`|CreateWidget` "/Game/Blueprints/WBP_LosingScreen.WBP_LosingScreen_C" _returnvalue))
  (set `self.LosingScreenRef` _returnvalue_4)
  (bind _returnvalue_5 (`|CreateWidget` "/Game/Blueprints/WBP_WinningScreen.WBP_WinningScreen_C" _returnvalue))
  (set `self.WinningScreenRef` _returnvalue_5)
  (`UserWidget.AddToViewport` (`self.WinningScreenRef`) 0)
  (`UserWidget.AddToViewport` (`self.LosingScreenRef`) 0)
  (`KismetSystemLibrary.K2_SetTimer` null "CheckIfDashAndJumpAvailable" 0.1 true))

(event `self.ReceiveTick`
  (params (DeltaSeconds :type "Float (single-precision)"))
  (set `self.JumpTimer` (+ (`self.JumpTimer`) DeltaSeconds)))

(event `InputAction|AttachLine`
  (params (Key :type "Key Structure"))
  (bind _returnvalue (`GameplayStatics.GetPlayerController` 0))
  (bind _returnvalue_2 (`self.K2_GetActorLocation`))
  (bind _returnvalue_x (`KismetMathLibrary.BreakVector` (`self.K2_GetActorLocation`)))
  (bind (_locationx _locationy) (`PlayerController.GetMousePosition` _returnvalue))
  (bind _cable (`/Game/Blueprints/Rope.Cable` (`self.Rope`)))
  (bind (_worldposition _worlddirection) (`GameplayStatics.DeprojectScreenToWorld` _returnvalue (`KismetMathLibrary.MakeVector2D` _locationx _locationy)))
  (bind (_returnvalue_x_2 _returnvalue_y _returnvalue_z) (`KismetMathLibrary.BreakVector` (+ _worldposition (* _worlddirection (`SpringArmComponent.TargetArmLength` (`self.CameraBoom`))))))
  (bind (_returnvalue_x_3 _returnvalue_y_2 _returnvalue_z_2) (`KismetMathLibrary.BreakVector` (+ _returnvalue_2 (* (`KismetMathLibrary.GetDirectionUnitVector` _returnvalue_2 (`KismetMathLibrary.MakeVector` 0.0 _returnvalue_y _returnvalue_z)) (`self.Raycasting distance`)))))
  (:`Pressed`
    (if (not (`self.Hanging`))
      (bind (_outhit _returnvalue_3) (`KismetSystemLibrary.LineTraceSingle` :`Start` _returnvalue_2 :`End` (`KismetMathLibrary.MakeVector` _returnvalue_x _returnvalue_y_2 _returnvalue_z_2) :`TraceChannel` "TraceTypeQuery1" :`DrawDebugType` "Persistent"))
      (if _returnvalue_3
        (for _array_element (`ActorComponent.ComponentTags` (`.HitComponent` (`GameplayStatics.BreakHitResult` _outhit)))
          _)
        (if (== _array_element "Attachable")
          (bind (_returnvalue_roll _returnvalue_pitch _returnvalue_yaw) (`KismetMathLibrary.BreakRotator` (`KismetMathLibrary.MakeRotFromY` (`KismetMathLibrary.GetDirectionUnitVector` (`self.K2_GetActorLocation`) (`.Location` (`GameplayStatics.BreakHitResult` _outhit))))))
          (bind _returnvalue_4 (`|SpawnActorFromClass` "/Game/Blueprints/Rope.Rope_C" (`KismetMathLibrary.MakeTransform` (`.Location` (`GameplayStatics.BreakHitResult` _outhit)) (`KismetMathLibrary.MakeRotator` _returnvalue_roll _returnvalue_pitch _returnvalue_yaw)) "Undefined" "OverrideRootScale" null null))
          (set `self.Rope` _returnvalue_4)
          (if (not (`self.Hanging`))
            (set `CableComponent.CableLength` (`KismetMathLibrary.Vector_Distance` (`self.K2_GetActorLocation`) (`.Location` (`GameplayStatics.BreakHitResult` _outhit))) _cable)
            (`CableComponent.SetAttachEndTo` _cable (`GameplayStatics.GetPlayerPawn` 0) "None" "None")
            (`SceneComponent.SetVisibility` _cable true false)
            (`SceneComponent.K2_AttachToComponent` (`self.Mesh`) (`/Game/Blueprints/Rope.CableEnd` (`self.Rope`)) "None" "KeepWorld" "KeepWorld" "KeepWorld" true)
            (set `self.Hanging` true)
            (set `self.IsSwinging` true)))))))

(event `InputAction|Jump`
  (params (Key :type "Key Structure"))
  (bind (_returnvalue_x _returnvalue_y) (`KismetMathLibrary.BreakVector` (`self.K2_GetActorLocation`)))
  (bind (_returnvalue_x_2 _returnvalue_y_2) (`KismetMathLibrary.BreakVector` (`SceneComponent.K2_GetComponentLocation` (`Actor.RootComponent` (`self.Rope`)))))
  (:`Pressed`
    (if (`self.Hanging`)
      (`SceneComponent.K2_DetachFromComponent` (`self.Mesh`) "KeepWorld" "KeepWorld" "KeepWorld" true :!label _label)
      (if (< _returnvalue_y_2 _returnvalue_y)
        (`PrimitiveComponent.AddForce` (`self.Mesh`) (0.0 2000.0 400.0) "None" true)
        (else
          (`PrimitiveComponent.AddForce` (`self.Mesh`) (0.0 -2000.0 400.0) "None" true)))
      (`KismetSystemLibrary.Delay` 0.2)
      (set `self.Hanging` false)
      (set `self.IsSwinging` false)
      (`self.K2_DestroyActor` (`self.Rope`))
      (elif (< (`self.JumpCooldown`) (`self.JumpTimer`))
        (`PrimitiveComponent.AddImpulse` (`self.Mesh`) (0.0 0.0 500.0) "None" true)
        (set `self.JumpTimer` 0.0)))))

(event `self.Detach`
  (goto _label))

(fn `CheckIfDashAndJumpAvailable`
  (bind _playerhud (`self.PlayerHud`))
  (bind _dashability (`self.DashAbility`))
  (bind _playerhud_2 (`self.PlayerHud`))
  (if (> (`self.JumpTimer`) (`self.JumpCooldown`))
    (`/Game/Blueprints/WBP_PlayerHUD.JumpAvalaible` _playerhud)
    (else
      (`/Game/Blueprints/WBP_PlayerHUD.JumpNotAvalaible` _playerhud)))
  (if (> (`DashAbility.Timer` _dashability) (`DashAbility.Cooldown` _dashability))
    (`/Game/Blueprints/WBP_PlayerHUD.DashAvalaible` _playerhud_2)
    (else
      (`/Game/Blueprints/WBP_PlayerHUD.DashNotAvalaible` _playerhud_2))))

(fn `isPlayer`
  (returns (`Yes/No` :type Boolean))
  (return false))

(fn `UserConstructionScript`)